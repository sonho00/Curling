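; BP_Pawn is the player pawn for a turn-based stone-launching game with a charge-to-shoot control.
; V spawns a Stone at a fixed point and tints it red or yellow through a dynamic material, flipping Turn each time.
; Holding G times the charge, shown on the BP_Widget HUD every tick.
; Releasing G sets the latest stone's physics velocity to MaxVelocity scaled by Percent, the hold time capped at MaxTime.
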(event `self.ReceiveBeginPlay`
  (bind _returnvalue (`|CreateWidget` "/Game/Blueprints/BP_Widget.BP_Widget_C"))
  (bind _output_get (set `self.HUD` _returnvalue))
  (`UserWidget.AddToViewport` _output_get 0))

(event `Key|V`
  (params (Key :type "Key Structure"))
  (:`Pressed`
    (bind _returnvalue (`|SpawnActorFromClass` "/Game/Blueprints/Stone.Stone_C" (`KismetMathLibrary.MakeTransform` (-5700.0 0.0 100.0)) "Undefined" "MultiplyWithRoot" null null))
    (bind _output_get (set `self.Stone` _returnvalue))
    (bind _returnvalue_2 (`PrimitiveComponent.CreateDynamicMaterialInstance` (`StaticMeshActor.StaticMeshComponent` _output_get) 0 "/Game/Materials/Stone.Stone" "None"))
    (if (`self.Turn`)
      (`MaterialInstanceDynamic.SetVectorParameterValue` _returnvalue_2 "Color" (struct :`R` 1.0 :`A` 1.0))
      (set `self.Turn` false)
      (else
        (`MaterialInstanceDynamic.SetVectorParameterValue` _returnvalue_2 "Color" (struct :`R` 1.0 :`G` 1.0 :`A` 1.0))
        (set `self.Turn` true)))))

(event `Key|G`
  (params (Key :type "Key Structure"))
  (:`Pressed`
    (set `self.PressedTime` (`GameplayStatics.GetTimeSeconds`)))
  (:`Released`
    (`PrimitiveComponent.SetPhysicsLinearVelocity` (`StaticMeshActor.StaticMeshComponent` (`self.Stone`)) (* (`self.MaxVelocity`) (`self.Percent`)) false "None")
    (set `self.PressedTime` 0.0)))

(event `self.ReceiveTick`
  (params (DeltaSeconds :type "Float (single-precision)"))
  (if (!= (`self.PressedTime`) 0.0)
    (set `/Game/Blueprints/BP_Widget.Velocity` (`self.Percent`) (`self.HUD`))))

(fn `UserConstructionScript`)